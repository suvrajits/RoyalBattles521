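; Enemy tower actor that sets its mesh and health from an Archer, Ballista or Cannon type.
; A sphere overlap sets damage by AI faction class and starts a looping ApplyDamage timer, with no stop on overlap end.
; Each tick lowers health and updates the widget health bar.
; At zero health it destroys itself, increments the GameState count, and triggers a win at three towers or when no Enemy_King-tagged actor remains.
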(event OnComponentBeginOverlap(Sphere)
  (params (OverlappedComponent :type Primitive%20Component%20Object%20Reference) (OtherActor :type Actor%20Object%20Reference) (OtherComp :type Primitive%20Component%20Object%20Reference) (OtherBodyIndex :type Integer) (bFromSweep :type Boolean) (SweepResult :type Hit%20Result%20Structure%20%28by%20ref%29))
  (bind _damageamount (CallFunction|GetAIDamage OtherActor))
  (Variables|Default|SetDamageAmount _damageamount)
  (Utilities|Time|SetTimerbyFunctionName 0 "ApplyDamage" 1.0 true))

(event EventBeginPlay
  (CallFunction|SetTowerProperties))

(fn ConstructionScript)

(fn SetTowerProperties
  (bind _towermesh (Variables|Default|GetTowerMesh))
  (switch Utilities|FlowControl|Switch|SwitchonE_TowerType (Variables|Default|GetTowerType)
    (:NewEnumerator0
      (Variables|Default|SetTowerHealth 1e+03)
      (Components|StaticMesh|SetStaticMesh _towermesh (Variables|Default|GetArcherMesh)))
    (:NewEnumerator1
      (Variables|Default|SetTowerHealth 1.5e+03)
      (Components|StaticMesh|SetStaticMesh _towermesh (Variables|Default|GetBallistaMesh)))
    (:NewEnumerator2
      (Variables|Default|SetTowerHealth 2e+03)
      (Components|StaticMesh|SetStaticMesh _towermesh (Variables|Default|GetCannonMesh)))))

(fn ApplyDamage
  (bind _output_get (Variables|Default|SetTowerHealth (- (Variables|Default|GetTowerHealth) (Variables|Default|GetDamageAmount))))
  (CallFunction|UpdateHealthUI)
  (if (<= _output_get 0.0)
    (CallFunction|DestroyTower)
    (else
      (CallFunction|UpdateHealthUI))))

(fn UpdateHealthUI
  (bind _asw_tower_health_bar (Utilities|Casting|CastToW_TowerHealthBar (UserInterface|GetUserWidgetObject (Variables|Default|GetHealthBarWidget))))
  (Default|SetHealthData _asw_tower_health_bar (Variables|Default|GetTowerHealth) (Variables|Default|GetMaxHealth)))

(fn DestroyTower
  (Actor|DestroyActor)
  (bind _asbp_game_state (Utilities|Casting|CastToBP_GameState (Game|GetGameState)))
  (bind _output_get (Variables|/Game/GameState/BP_GameState.BP_GameState_C|SetEnemyTowersDestroyed _asbp_game_state (+ (Variables|/Game/GameState/BP_GameState.BP_GameState_C|GetEnemyTowersDestroyed _asbp_game_state) 1)))
  (if (>= _output_get 3)
    (if (not (Variables|/Game/GameState/BP_GameState.BP_GameState_C|GetisGameOver _asbp_game_state)) :!label _label
      (Default|GameOverEvent _asbp_game_state "You Win")
      (Variables|/Game/GameState/BP_GameState.BP_GameState_C|SetisGameOver _asbp_game_state true))
    (else
      (bind _outactors (Actor|GetAllActorswithTag "Enemy_King"))
      (if (not (> (Utilities|Array|Length _outactors) 0))
        (goto _label)))))

(fn GetAIDamage
  (params (AIActor :type Actor%20Object%20Reference))
  (Utilities|Casting|CastToPC_AI_Viking AIActor
    (:then
      (return 7e+01))
    (:CastFailed
      (Utilities|Casting|CastToPC_AI_Egyptian AIActor
        (:then
          (return 4e+01))
        (:CastFailed
          (Utilities|Casting|CastToPC_AI_Egyptian AIActor
            (:then
              (return 9e+01))
            (:CastFailed
              (Utilities|Casting|CastToPC_AI_Mayan AIActor
                (:then
                  (return 5e+01))
                (:CastFailed
                  (return 0.0))))))))))