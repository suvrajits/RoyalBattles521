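; Game state for a tower match that holds player and enemy mana, destroyed-tower counts and the game-over flow.
; Looping timers started at BeginPlay regenerate both mana pools and clear the IsSpawned flag at an interval randomized once.
; Consume functions spend mana when affordable, reading stored Amount variables rather than their ManaCost inputs.
; GameOverEvent shows the result widget and loads the main menu after a delay, while ResetGameState restores defaults.
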(event EventBeginPlay
  (Utilities|Time|SetTimerbyFunctionName 0 "RegenerateMana" 1.0 true)
  (Utilities|Time|SetTimerbyFunctionName 0 "RegenerateEnemyMana" 1.0 true)
  (Utilities|Time|SetTimerbyFunctionName 0 "CheckAndResetIsSpawned" (Math|Random|RandomFloatinRange 2.0 5.0) true))

(fn ConstructionScript)

(fn RegenerateMana
  (bind _output_get (Variables|Default|SetNewMana (+ (Variables|Default|GetPlayerMana) (Variables|Default|GetManaRegenRate))))
  (bind _output_get_2 (Variables|Default|SetPlayerMana (Math|Float|Clamp(Float) _output_get 0.0 (Variables|Default|GetPlayerMaxMana))))
  (Development|PrintString (Utilities|String|ToString(Float) _output_get_2)))

(fn ConsumeMana
  (params (ManaCost :type Float%20%28double-precision%29))
  (if (>= (Variables|Default|GetPlayerMana) (Variables|Default|GetAmount))
    (bind _output_get (Variables|Default|SetNewMana (- (Variables|Default|GetPlayerMana) (Variables|Default|GetAmount))))
    (Variables|Default|SetPlayerMana (Math|Float|Clamp(Float) _output_get 0.0 (Variables|Default|GetPlayerMaxMana)))
    (bind _output_get_2 (Variables|Default|SetbSuccess true))
    (return _output_get_2)
    (else
      (bind _output_get_3 (Variables|Default|SetbSuccess false))
      (return _output_get_3))))

(fn RegenerateEnemyMana
  (bind _output_get (Variables|Default|SetEnemyNewMana (+ (Variables|Default|GetEnemyMana) (Variables|Default|GetEnemyManaRegenRate))))
  (bind _output_get_2 (Variables|Default|SetEnemyMana (Math|Float|Clamp(Float) _output_get 0.0 (Variables|Default|GetEnemyMaxMana))))
  (Development|PrintString (Utilities|String|ToString(Float) _output_get_2)))

(fn ConsumeEnemyMana
  (params (ManaCost :type Float%20%28double-precision%29))
  (if (>= (Variables|Default|GetEnemyMana) (Variables|Default|GetEnemyAmount))
    (bind _output_get (Variables|Default|SetEnemyNewMana (- (Variables|Default|GetEnemyMana) (Variables|Default|GetEnemyAmount))))
    (Variables|Default|SetEnemyMana (Math|Float|Clamp(Float) _output_get 0.0 (Variables|Default|GetEnemyMaxMana)))
    (bind _output_get_2 (Variables|Default|SetbEnemySuccess true))
    (return _output_get_2)
    (else
      (bind _output_get_3 (Variables|Default|SetbEnemySuccess false))
      (return _output_get_3))))

(fn ResetGameState
  (Variables|Default|SetPlayerMana 1e+01)
  (Variables|Default|SetPlayerMaxMana 1e+01)
  (Variables|Default|SetManaRegenRate 1.0)
  (Variables|Default|SetNewMana 0.0)
  (Variables|Default|SetAmount 0.0)
  (Variables|Default|SetbSuccess false)
  (Variables|Default|SetEnemyMana 1e+01)
  (Variables|Default|SetEnemyMaxMana 1e+01)
  (Variables|Default|SetEnemyManaRegenRate 1.0)
  (Variables|Default|SetEnemyNewMana 0.0)
  (Variables|Default|SetEnemyAmount 0.0)
  (Variables|Default|SetbEnemySuccess false)
  (Variables|Default|SetisGameOver false)
  (Variables|Default|SetEnemyTowersDestroyed 0)
  (Variables|Default|SetPlayerTowersDestroyed 0)
  (Development|PrintString "Resetting all variables")
  (Variables|Default|SetGameOverMessage ""))

(fn GameOverEvent
  (params (ResultText :type String))
  (Variables|Default|SetGameOverMessage (Utilities|Text|ToText(String) ResultText))
  (bind _returnvalue (UserInterface|CreateWidget "/Game/UI/UI_GameOver.UI_GameOver_C"))
  (UserInterface|Viewport|AddtoViewport _returnvalue 0)
  (Utilities|Time|SetTimerbyFunctionName 0 "OpenMainMenu" 5.0))

(fn OpenMainMenu
  (Game|OpenLevel(byName) "MainMenuLevel"))

(fn CheckandResetIsSpawned
  (if (Variables|Default|GetisSpawned)
    (Variables|Default|SetisSpawned false)))