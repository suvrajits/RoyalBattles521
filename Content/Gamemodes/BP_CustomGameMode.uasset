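; Custom game mode that puts the UI_NewCanvas widget on screen at BeginPlay and tracks the towers in the level.
; GetActiveTowers clears the ActiveTowers array and refills it with every BP_Tower actor found in the world.
; The per-player ownership check is left unconnected, so the Player argument does not filter the result.
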(event Custom|GetActiveTowers
  (params (Player :type Byte))
  (Utilities|Array|Clear (Variables|Default|GetActiveTowers))
  (bind _outactors (Actor|GetAllActorsOfClass "/Game/Tower/BP_Tower.BP_Tower_C"))
  (for _array_element _outactors
    (if true
      (Utilities|Array|Add (Variables|Default|GetActiveTowers) _array_element))))

(event EventBeginPlay
  (bind _returnvalue (UserInterface|CreateWidget "/Game/UI/UI_NewCanvas.UI_NewCanvas_C"))
  (UserInterface|Viewport|AddtoViewport _returnvalue 0))

(fn ConstructionScript)