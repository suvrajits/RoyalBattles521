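; Enemy spawn point that periodically tries to spawn a random AI enemy, paid for from enemy mana.
; A looping timer, initially randomized, picks a class from EnemyClasses and maps its name to a DT_CardData row for the mana cost.
; If GameState's IsSpawned is false and ConsumeEnemyMana succeeds, it spawns at any random spawn point, sets IsSpawned and resets the timer to a fixed interval.
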(event EventBeginPlay
  (Utilities|Time|SetTimerbyFunctionName 0 "SpawnEnemy" (Math|Random|RandomFloatinRange 3.0 7.0) true))

(fn ConstructionScript)

(fn SpawnEnemy
  (bind _enemyclasses (Variables|Default|GetEnemyClasses))
  (bind _outactors (Actor|GetAllActorsOfClass "BP_EnemySpawnPoint_C"))
  (bind _output_get (Variables|Default|SetSelectedEnemyClass (Utilities|Array|Get(acopy) _enemyclasses (Math|Random|RandomIntegerinRange 0 (- (Utilities|Array|Length _enemyclasses) 1)))))
  (switch name (Utilities|String|StringToName (Utilities|GetClassDisplayName _output_get))
    (:EC_AI_Mayan_C
      (Variables|Default|SetDB_RowName "Mayan"))
    (:EC_AI_Egyptian_C
      (Variables|Default|SetDB_RowName "Egyptian"))
    (:EC_AI_Viking_C
      (Variables|Default|SetDB_RowName "Viking"))
    (:EC_AI_Indian_C
      (Variables|Default|SetDB_RowName "Indian")))
  (bind _success (CallFunction|CheckEnemyCanDrop))
  (if _success
    (AI|SpawnAIFromClass _output_get 0 (Transformation|GetActorLocation (Utilities|Array|Get(acopy) _outactors (Math|Random|RandomIntegerinRange 0 (- (Utilities|Array|Length _outactors) 1)))) "0, 0, 0" false 0)
    (bind _asbp_game_state (Utilities|Casting|CastToBP_GameState (Game|GetGameState)))
    (Variables|/Game/GameState/BP_GameState.BP_GameState_C|SetisSpawned _asbp_game_state true)
    (Utilities|Time|SetTimerbyFunctionName 0 "SpawnEnemy" 2.0 true)))

(fn CheckEnemyCanDrop
  (bind _db_rowname (Variables|Default|GetDB_RowName))
  (bind _returnvalue (Utilities|GetDataTableRow "/Game/Datasstructure/DT_CardData.DT_CardData" (Utilities|String|StringToName _db_rowname))
    (:then
      (bind _asbp_game_state (Utilities|Casting|CastToBP_GameState (Game|GetGameState)))
      (bind _output_get (Variables|/Game/GameState/BP_GameState.BP_GameState_C|SetEnemyAmount _asbp_game_state (.ManaCost (Utilities|Struct|BreakST_CardData _returnvalue))))
      (bind _asbp_game_state_2 (Utilities|Casting|CastToBP_GameState (Game|GetGameState)))
      (if (not (Variables|/Game/GameState/BP_GameState.BP_GameState_C|GetisSpawned _asbp_game_state_2))
        (bind _success (Default|ConsumeEnemyMana _asbp_game_state _output_get))
        (return _success)))
    (:RowNotFound
      (Development|PrintString _db_rowname)
      (Development|PrintString "Not found in db"))))

(fn CanSpawn)