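; PC_Troup is a troop pawn that walks toward a tower when play begins.
; BeginPlay gets a single BP_Tower via GetActorOfClass and issues AI MoveTo with it as the target.
; A separate FindNearestTower function loops over all towers, storing and printing each one closer than the current NearestDistance, but nothing in this Blueprint calls it, so movement ignores proximity.
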(event EventBeginPlay
  (bind _returnvalue (Actor|GetActorOfClass "/Game/Tower/BP_Tower.BP_Tower_C"))
  (AI|AIMoveTo self "0, 0, 0" _returnvalue 1e+02 false))

(fn ConstructionScript)

(fn FindNearestTower
  (bind _outactors (Actor|GetAllActorsOfClass "/Game/Tower/BP_Tower.BP_Tower_C"))
  (for _array_element _outactors
    (if (< (Math|Vector|Distance(Vector) (Transformation|GetActorLocation) (Transformation|GetActorLocation _array_element)) (Variables|Default|GetNearestDistance))
      (bind _output_get (Variables|Default|SetNearestTower _array_element))
      (Variables|Default|SetNearestDistance (Math|Vector|Distance(Vector) (Transformation|GetActorLocation) (Transformation|GetActorLocation _array_element)))
      (Development|PrintString (Utilities|GetDisplayName _output_get)))))