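; AI-driven Viking unit that, on BeginPlay, heads for a tagged bridge, then advances on the enemy queen paired with it.
; Distances to both bridges pick the nearer route through chained AIMoveTo calls, though both Sequence pins run the comparison, the first before Bridge2's data is set.
; A card type can be stored, but UpdateSkeletalMesh only prints the matching civilization name, without changing the mesh.
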(event EventBeginPlay
  (Utilities|FlowControl|Sequence
    (:then_0
      (bind _outactors (Actor|GetAllActorswithTag "Bridge1"))
      (bind _output_get (Variables|Default|SetBridge1Ref (Utilities|Array|Get(acopy) _outactors)))
      (bind _output_get_2 (Variables|Default|SetDistance1 (Transformation|GetDistanceTo _output_get))))
    (:then_1
      (bind _outactors_2 (Actor|GetAllActorswithTag "Bridge2"))
      (bind _output_get_3 (Variables|Default|SetBridge2Ref (Utilities|Array|Get(acopy) _outactors_2)))
      (bind _output_get_4 (Variables|Default|SetDistance2 (Transformation|GetDistanceTo _output_get_3)))))
  (if (> _output_get_2 _output_get_4)
    (AI|AIMoveTo self "0, 0, 0" (Variables|Default|GetBridge2Ref) 1e+01 false
      (:OnSuccess
        (bind _outactors_3 (Actor|GetAllActorswithTag "Enemy_QueenB"))
        (AI|AIMoveTo self "0, 0, 0" (Utilities|Array|Get(acopy) _outactors_3) 5.0 false)))
    (else
      (AI|AIMoveTo self "0, 0, 0" (Variables|Default|GetBridge1Ref) 1e+01 false
        (:OnSuccess
          (bind _outactors_4 (Actor|GetAllActorswithTag "Enemy_QueenA"))
          (AI|AIMoveTo self "0, 0, 0" (Utilities|Array|Get(acopy) _outactors_4) 5.0 false))))))

(fn ConstructionScript)

(fn SettingCardType
  (params (NewCardType :type Byte :default 0))
  (Variables|Default|SetLatestCardType NewCardType))

(fn UpdateSkeletalMesh
  (switch Utilities|FlowControl|Switch|Switchon (Variables|Default|GetLatestCardType)
    (:NewEnumerator0
      (Development|PrintString "Hello: Egyptian"))
    (:NewEnumerator1
      (Development|PrintString "Hello: Mayan"))
    (:NewEnumerator2
      (Development|PrintString "Hello: Viking"))
    (:NewEnumerator3
      (Development|PrintString "Hello: Indian"))))