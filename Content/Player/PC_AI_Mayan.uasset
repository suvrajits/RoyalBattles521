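; PC_AI_Mayan is an AI-moved pawn that walks toward a randomly chosen BP_Tower when play begins.
; BeginPlay calls UpdateSkeletalMesh, then issues AIMoveTo, printing on arrival, or after a short delay on failure without actually retrying.
; SettingCardType stores the card type as an enum, which UpdateSkeletalMesh switches on, though that switch has no cases wired.
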(event EventBeginPlay
  (CallFunction|UpdateSkeletalMesh)
  (bind _outactors (Actor|GetAllActorsOfClass "/Game/Tower/BP_Tower.BP_Tower_C"))
  (AI|AIMoveTo self "0, 0, 0" (Utilities|Array|Get(acopy) _outactors (Math|Random|RandomIntegerinRange 0 (- (Utilities|Array|Length _outactors) 1))) 1e+02 true
    (:OnSuccess
      (Development|PrintString "Reached Tower"))
    (:OnFail
      (Utilities|FlowControl|Delay 0.5)
      (Development|PrintString "retrying to move"))))

(fn ConstructionScript)

(fn SettingCardType
  (params (NewCardType :type Byte :default 0))
  (Variables|Default|SetLatestCardType (Utilities|Enum|ByteToEnumE_CardType NewCardType)))

(fn UpdateSkeletalMesh
  (switch Utilities|FlowControl|Switch|SwitchonE_CardType (Variables|Default|GetLatestCardType)))