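; Player-side Indian AI unit that pushes a lane toward the enemy towers in a card-based tower battle.
; It picks a bridge by distance, moves to that lane's Queen tower, polls until it is gone, then heads for the King.
; Overlapping enemy units stop it and set class-based damage that a looping timer subtracts from its own health, updating the health bar.
; When that enemy becomes invalid, a flag checked on Tick resumes movement.
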(event OnComponentBeginOverlap(Sphere)
  (params (OverlappedComponent :type Primitive%20Component%20Object%20Reference) (OtherActor :type Actor%20Object%20Reference) (OtherComp :type Primitive%20Component%20Object%20Reference) (OtherBodyIndex :type Integer) (bFromSweep :type Boolean) (SweepResult :type Hit%20Result%20Structure%20%28by%20ref%29))
  (Variables|Default|SetCurrentTarget OtherActor)
  (bind _damageamount (CallFunction|GetPlayerDamage OtherActor))
  (Variables|Default|SetDamageAmount _damageamount)
  (Utilities|Time|SetTimerbyFunctionName 0 "ReceiveDamage" 1.0 true)
  (if (Variables|Default|GetCanResumeMovement)
    (Variables|Default|SetCanResumeMovement false)
    (if (Variables|Default|GethasCrossedBridge)
      (if (Utilities|Enum|Equal(Enum) (Variables|Default|GetQueenTowerTag) "Enemy_QueenB")
        (Variables|Default|SetQueenTowerTag "Enemy_QueenB" :!label _label)
        (Variables|Default|SethasCrossedBridge true)
        (bind _validtarget (CallFunction|CheckValidTarget))
        (AI|AIMoveTo self "0, 0, 0" _validtarget 1e+01 false
          (:OnSuccess
            (bind _isalive (CallFunction|IsTowerBAlive :!label _label_2))
            (if _isalive
              (Utilities|FlowControl|Delay 0.5)
              (goto _label_2)
              (else
                (bind _outactors (Actor|GetAllActorswithTag "Enemy_King"))
                (bind _output_get (Variables|Default|SetNearestTower (Utilities|Array|Get(acopy) _outactors)))
                (AI|AIMoveTo self "0, 0, 0" _output_get 1e+01 false)))))
        (else
          (Variables|Default|SetQueenTowerTag "Enemy_QueenA" :!label _label_3)
          (Variables|Default|SethasCrossedBridge true)
          (bind _validtarget_2 (CallFunction|CheckValidTarget))
          (bind _output_get_2 (Variables|Default|SetNearestTower _validtarget_2))
          (AI|AIMoveTo self "0, 0, 0" _output_get_2 1e+01 false
            (:OnSuccess
              (bind _isalive_2 (CallFunction|IsTowerAAlive :!label _label_4))
              (if _isalive_2
                (Utilities|FlowControl|Delay 0.5)
                (goto _label_4)
                (else
                  (bind _outactors_2 (Actor|GetAllActorswithTag "Enemy_King"))
                  (bind _output_get_3 (Variables|Default|SetNearestTower (Utilities|Array|Get(acopy) _outactors_2)))
                  (AI|AIMoveTo self "0, 0, 0" _output_get_3 1e+01 false)))))))
      (elif (> (stale EventBeginPlay _output_get_2) (stale EventBeginPlay _output_get_4))
        (AI|AIMoveTo self "0, 0, 0" (Variables|Default|GetBridge2Ref) 1e+01 false
          (:OnSuccess
            (goto _label)))
        (else
          (AI|AIMoveTo self "0, 0, 0" (Variables|Default|GetBridge1Ref) 1e+01 false
            (:OnSuccess
              (goto _label_3))))))))

(event EventBeginPlay
  (Utilities|FlowControl|Sequence
    (:then_0
      (bind _outactors (Actor|GetAllActorswithTag "Bridge1"))
      (bind _output_get (Variables|Default|SetBridge1Ref (Utilities|Array|Get(acopy) _outactors)))
      (bind _output_get_2 (Variables|Default|SetDistance1 (Transformation|GetDistanceTo _output_get))))
    (:then_1
      (bind _outactors_2 (Actor|GetAllActorswithTag "Bridge2"))
      (bind _output_get_3 (Variables|Default|SetBridge2Ref (Utilities|Array|Get(acopy) _outactors_2)))
      (bind _output_get_4 (Variables|Default|SetDistance2 (Transformation|GetDistanceTo _output_get_3)))))
  (if (> _output_get_2 _output_get_4)
    (AI|AIMoveTo self "0, 0, 0" (Variables|Default|GetBridge2Ref) 1e+01 false
      (:OnSuccess
        (Variables|Default|SetQueenTowerTag "Enemy_QueenB")
        (Variables|Default|SethasCrossedBridge true)
        (bind _validtarget (CallFunction|CheckValidTarget))
        (AI|AIMoveTo self "0, 0, 0" _validtarget 1e+01 false
          (:OnSuccess
            (bind _isalive (CallFunction|IsTowerBAlive :!label _label))
            (if _isalive
              (Utilities|FlowControl|Delay 0.5)
              (goto _label)
              (else
                (bind _outactors_3 (Actor|GetAllActorswithTag "Enemy_King"))
                (bind _output_get_5 (Variables|Default|SetNearestTower (Utilities|Array|Get(acopy) _outactors_3)))
                (AI|AIMoveTo self "0, 0, 0" _output_get_5 1e+01 false)))))))
    (else
      (AI|AIMoveTo self "0, 0, 0" (Variables|Default|GetBridge1Ref) 1e+01 false
        (:OnSuccess
          (Variables|Default|SetQueenTowerTag "Enemy_QueenA")
          (Variables|Default|SethasCrossedBridge true)
          (bind _validtarget_2 (CallFunction|CheckValidTarget))
          (bind _output_get_6 (Variables|Default|SetNearestTower _validtarget_2))
          (AI|AIMoveTo self "0, 0, 0" _output_get_6 1e+01 false
            (:OnSuccess
              (bind _isalive_2 (CallFunction|IsTowerAAlive :!label _label_2))
              (if _isalive_2
                (Utilities|FlowControl|Delay 0.5)
                (goto _label_2)
                (else
                  (bind _outactors_4 (Actor|GetAllActorswithTag "Enemy_King"))
                  (bind _output_get_7 (Variables|Default|SetNearestTower (Utilities|Array|Get(acopy) _outactors_4)))
                  (AI|AIMoveTo self "0, 0, 0" _output_get_7 1e+01 false))))))))))

(event EventTick
  (params (DeltaSeconds :type Float%20%28single-precision%29))
  (if (Variables|Default|GetCanResumeMovement)
    (Variables|Default|SetCanResumeMovement false)
    (if (Variables|Default|GethasCrossedBridge)
      (if (Utilities|Enum|Equal(Enum) (Variables|Default|GetQueenTowerTag) "Enemy_QueenB")
        (Variables|Default|SetQueenTowerTag "Enemy_QueenB" :!label _label)
        (Variables|Default|SethasCrossedBridge true)
        (bind _validtarget (CallFunction|CheckValidTarget))
        (AI|AIMoveTo self "0, 0, 0" _validtarget 1e+01 false
          (:OnSuccess
            (bind _isalive (CallFunction|IsTowerBAlive :!label _label_2))
            (if _isalive
              (Utilities|FlowControl|Delay 0.5)
              (goto _label_2)
              (else
                (bind _outactors (Actor|GetAllActorswithTag "Enemy_King"))
                (bind _output_get (Variables|Default|SetNearestTower (Utilities|Array|Get(acopy) _outactors)))
                (AI|AIMoveTo self "0, 0, 0" _output_get 1e+01 false)))))
        (else
          (Variables|Default|SetQueenTowerTag "Enemy_QueenA" :!label _label_3)
          (Variables|Default|SethasCrossedBridge true)
          (bind _validtarget_2 (CallFunction|CheckValidTarget))
          (bind _output_get_2 (Variables|Default|SetNearestTower _validtarget_2))
          (AI|AIMoveTo self "0, 0, 0" _output_get_2 1e+01 false
            (:OnSuccess
              (bind _isalive_2 (CallFunction|IsTowerAAlive :!label _label_4))
              (if _isalive_2
                (Utilities|FlowControl|Delay 0.5)
                (goto _label_4)
                (else
                  (bind _outactors_2 (Actor|GetAllActorswithTag "Enemy_King"))
                  (bind _output_get_3 (Variables|Default|SetNearestTower (Utilities|Array|Get(acopy) _outactors_2)))
                  (AI|AIMoveTo self "0, 0, 0" _output_get_3 1e+01 false)))))))
      (elif (> (stale EventBeginPlay _output_get_2) (stale EventBeginPlay _output_get_4))
        (AI|AIMoveTo self "0, 0, 0" (Variables|Default|GetBridge2Ref) 1e+01 false
          (:OnSuccess
            (goto _label)))
        (else
          (AI|AIMoveTo self "0, 0, 0" (Variables|Default|GetBridge1Ref) 1e+01 false
            (:OnSuccess
              (goto _label_3))))))))

(fn ConstructionScript)

(fn SettingCardType
  (params (NewCardType :type Byte :default 0))
  (bind _output_get (Variables|Default|SetLatestCardType (Utilities|Enum|ByteToEnumE_CardType NewCardType)))
  (Development|PrintString "Card Set:")
  (Development|PrintString (Utilities|String|EnumtoString _output_get)))

(fn UpdateSkeletalMesh
  (switch Utilities|FlowControl|Switch|SwitchonE_CardType (Variables|Default|GetLatestCardType)
    (:NewEnumerator0
      (Development|PrintString "Hello: Egyptian"))
    (:NewEnumerator1
      (Development|PrintString "Hello: Mayan"))
    (:NewEnumerator2
      (Development|PrintString "Hello: Viking"))
    (:NewEnumerator3
      (Development|PrintString "Hello: Indian"))))

(fn CheckValidTarget
  (bind _outactors (Actor|GetAllActorswithTag (Utilities|String|StringToName (Variables|Default|GetQueenTowerTag))))
  (if (> (Utilities|Array|Length _outactors) 0)
    (return (Utilities|Array|Get(acopy) _outactors))
    (else
      (bind _outactors_2 (Actor|GetAllActorswithTag "Enemy_King"))
      (if (> (Utilities|Array|Length _outactors_2) 0)
        (return (Utilities|Array|Get(acopy) _outactors_2))))))

(fn IsTowerAAlive
  (bind _outactors (Actor|GetAllActorswithTag "Enemy_QueenA"))
  (if (> (Utilities|Array|Length _outactors) 0)
    (return true)
    (else
      (return false))))

(fn IsTowerBAlive
  (bind _outactors (Actor|GetAllActorswithTag "Enemy_QueenB"))
  (if (> (Utilities|Array|Length _outactors) 0)
    (return true)
    (else
      (return false))))

(fn StartAttackTimer
  (Utilities|Time|SetTimerbyFunctionName 0 "PerformAttack" (Variables|Default|GetAttackRate) true))

(fn PerformAttack
  (bind _aspc_ai_indian (Utilities|Casting|CastToPC_AI_Indian (Variables|Default|GetTargetActor)))
  (CallFunction|ReceiveDamage _aspc_ai_indian))

(fn ReceiveDamage
  (Utilities|IsValid (Variables|Default|GetCurrentTarget)
    (:Is%20Valid
      (bind _output_get (Variables|Default|SetHealth (- (Variables|Default|GetHealth) (Variables|Default|GetDamageAmount))))
      (CallFunction|UpdateHealthUI)
      (if (<= _output_get 0.0)
        (Actor|DestroyActor)))
    (:Is%20Not%20Valid
      (Variables|Default|SetCurrentTarget 0)
      (Variables|Default|SetCanResumeMovement true)
      (Utilities|Time|ClearTimerbyFunctionName 0 "ReceiveDamage"))))

(fn GetPlayerDamage
  (params (AIActor :type Actor%20Object%20Reference))
  (Utilities|Casting|CastToEC_AI_Viking AIActor
    (:then
      (AI|Navigation|StopMovement (Pawn|GetController self))
      (return 35.0))
    (:CastFailed
      (Utilities|Casting|CastToEC_AI_Indian AIActor
        (:then
          (AI|Navigation|StopMovement (Pawn|GetController self))
          (return 2e+01))
        (:CastFailed
          (Utilities|Casting|CastToEC_AI_Egyptian AIActor
            (:then
              (AI|Navigation|StopMovement (Pawn|GetController self))
              (return 45.0))
            (:CastFailed
              (Utilities|Casting|CastToEC_AI_Mayan AIActor
                (:then
                  (AI|Navigation|StopMovement (Pawn|GetController self))
                  (return 25.0))
                (:CastFailed
                  (return 0.0))))))))))

(fn UpdateHealthUI
  (bind _aswbp_p_health_bar (Utilities|Casting|CastToWBP_P_HealthBar (UserInterface|GetUserWidgetObject (Variables|Default|GetHealthBarWidget))))
  (Default|SetHealthData _aswbp_p_health_bar (Variables|Default|GetHealth) (Variables|Default|GetMaxHealth)))