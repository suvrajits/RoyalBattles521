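; BP_EnemySpawner periodically spawns random AI enemies at spawn points placed in the level.
; BeginPlay starts a looping timer on SpawnEnemy, with an interval randomized once at startup.
; SpawnEnemy picks a random pawn class from EnemyClasses and spawns it at a random BP_EnemySpawnPoint, gathering all points on every call.
; The EnemySpawnPoint function is empty, with leftover selection logic left disconnected.
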(event EventBeginPlay
  (Utilities|Time|SetTimerbyFunctionName 0 "SpawnEnemy" (Math|Random|RandomFloatinRange 0.3 2.0) true))

(fn ConstructionScript)

(fn EnemySpawnPoint)

(fn SpawnEnemy
  (bind _enemyclasses (Variables|Default|GetEnemyClasses))
  (bind _outactors (Actor|GetAllActorsOfClass "/Game/Player/BP_EnemySpawnPoint.BP_EnemySpawnPoint_C"))
  (AI|SpawnAIFromClass (Utilities|Array|Get(acopy) _enemyclasses (Math|Random|RandomIntegerinRange 0 (- (Utilities|Array|Length _enemyclasses) 1))) 0 (Transformation|GetActorLocation (Utilities|Array|Get(acopy) _outactors (Math|Random|RandomIntegerinRange 0 (- (Utilities|Array|Length _outactors) 1)))) "0, 0, 0" false 0))