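; AI-controlled pawn that walks to a randomly chosen BP_Tower when play begins.
; BeginPlay picks the tower and issues a single AI MoveTo, printing on success or, after a short delay, a retry message on failure without moving again.
; A nearest-tower search and a manual movement-input step exist but never run, and MoveToTarget is an empty stub.
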(event EventBeginPlay
  (bind _outactors (Actor|GetAllActorsOfClass "/Game/Tower/BP_Tower.BP_Tower_C"))
  (AI|AIMoveTo self "0, 0, 0" (Utilities|Array|Get(acopy) _outactors (Math|Random|RandomIntegerinRange 0 (- (Utilities|Array|Length _outactors) 1))) 1e+02 true
    (:OnSuccess
      (Development|PrintString "Reached Tower"))
    (:OnFail
      (Utilities|FlowControl|Delay 0.5)
      (Development|PrintString "retrying to move"))))

(fn ConstructionScript)

(fn FindNearestTower
  (bind _outactors (Actor|GetAllActorsOfClass "/Game/Tower/BP_Tower.BP_Tower_C"))
  (for _array_element _outactors
    (if (< (Math|Vector|Distance(Vector) (Transformation|GetActorLocation) (Transformation|GetActorLocation _array_element)) (Variables|Default|GetNearestDistance))
      (bind _output_get (Variables|Default|SetNearestTower _array_element))
      (Variables|Default|SetNearestDistance (Math|Vector|Distance(Vector) (Transformation|GetActorLocation) (Transformation|GetActorLocation _array_element)))
      (Development|PrintString (Utilities|GetDisplayName _output_get)))))

(fn MovetoTarget)